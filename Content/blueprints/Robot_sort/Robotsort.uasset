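; Robot-sort actor that runs a command program from the UI, gliding a Paper sprite between five stones.
; CNext interprets the integer command stream through GlobalIter: loop start/end, size-based minimum, swap and assign to Temp.
; Loop and iterator stacks support nested loops, with each operand resolved as Temp or an iterator.
; Steps are reported to the UI; the stone-exchange chain in swap is disconnected, so it only moves the robot.
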(event `Error`
  (set `self.Message` "ERROR")
  (`/Game/blueprints/Robot_sort/UI/RobotWidgetBase.UpDate` (`self.UI`)))

(event `self.ReceiveBeginPlay`
  (set `self.Array` (`|MakeArray` (`self.Stone_1`) (`self.Stone_2`) (`self.Stone_3`) (`self.Stone_4`) (`self.Stone_5`))))

(event `Start`
  (set `self.GlobalIter` 0)
  (bind _output_get (set `self.Commands` (`/Game/blueprints/Robot_sort/UI/RobotWidgetBase.Commands` (`self.UI`))))
  (set `self.Message` "")
  (for _array_element _output_get
    (set `self.Message` (`KismetStringLibrary.Concat_StrStr` (`self.Message`) (`KismetStringLibrary.Conv_IntToString` _array_element))))
  (`/Game/blueprints/Robot_sort/UI/RobotWidgetBase.UpDate` (`self.UI`))
  (`self.CNext`))

(event `CNext`
  (if (>= (`self.GlobalIter`) (`KismetArrayLibrary.Array_Length` (`self.Commands`)))
    (`self.Error`)
    (else
      (`/Engine/EditorBlueprintResources/StandardMacros.IncrementInt` (`self.GlobalIter`)
        (:`  `
          (switch `int` (`|GetArrayItem` (`self.Commands`) (- (`self.GlobalIter`) 1))
            (:`0`
              (bind (_x _returnvalue) (`self.fEndLoop`))
              (if _returnvalue
                (bind _relativelocation_x (`KismetMathLibrary.BreakVector` (`SceneComponent.RelativeLocation` (`|GetArrayItem` (`self.Array`) _x))))
                (`self.MMove` _relativelocation_x
                  (:`Completed`
                    _)))
              (`self.CNext` :!label _label))
            (:`1`
              (bind _x_2 (`self.fCycle`))
              (bind _relativelocation_x_2 (`KismetMathLibrary.BreakVector` (`SceneComponent.RelativeLocation` (`|GetArrayItem` (`self.Array`) _x_2))))
              (`self.MMove` _relativelocation_x_2
                (:`Completed`
                  (goto _label))))
            (:`2`
              (`self.fMin`)
              (goto _label))
            (:`3`
              (`self.CSwap`))
            (:`4`
              (`self.fTEq`)
              (goto _label))))))))

(event `CSwap`
  (bind _relativelocation_x (`KismetMathLibrary.BreakVector` (`SceneComponent.RelativeLocation` (`|GetArrayItem` (`self.Array`) (`self.Var1`)))))
  (`|ExecutionSequence`
    (:`then_0`
      (bind _newparam (`self.IterOrConst`))
      (bind _output_get (set `self.Var1` _newparam))
      (set `self.Message` (`KismetStringLibrary.Concat_StrStr` "Меняет " (`KismetStringLibrary.Conv_IntToString` _output_get)))
      (`/Game/blueprints/Robot_sort/UI/RobotWidgetBase.UpDate` (`self.UI`)))
    (:`then_1`
      (bind _newparam_2 (`self.IterOrConst`))
      (bind _output_get_2 (set `self.Var2` _newparam_2))
      (set `self.Message` (`KismetStringLibrary.Concat_StrStr` " с " (`KismetStringLibrary.Conv_IntToString` _output_get_2)))
      (`/Game/blueprints/Robot_sort/UI/RobotWidgetBase.UpDate` (`self.UI`)))
    (:`then_2`
      (if (== (`self.Var1`) (`self.Var2`))
        (`self.CNext`)
        (else
          (`self.MMove` _relativelocation_x))))))

(fn `fCycle`
  (returns (X :type Integer))
  (locals (TempIt :type Integer))
  (bind _loopstack (`self.LoopStack`))
  (bind _globaliter (`self.GlobalIter`))
  (bind _tempit (`local.TempIt`))
  (bind _output (`|GetArrayItem` (`self.Commands`) (- _globaliter 1)))
  (bind _output_x (break `IntVector` (`|GetArrayItem` _loopstack (`KismetArrayLibrary.Array_LastIndex` _loopstack))))
  (bind _output_get (set `self.GlobalIter` (+ (stale _output_get) 3)))
  (switch `int` (`|GetArrayItem` (`self.Commands`) (- (`self.GlobalIter`) 3))
    (:`Default`
      (set `local.TempIt` (`|GetArrayItem` (`self.StackIter`) (`|GetArrayItem` (`self.Commands`) (- (`self.GlobalIter`) 2))) :!label _label))
    (:`-1`
      (set `local.TempIt` (`|GetArrayItem` (`self.Commands`) (- (`self.GlobalIter`) 2))))
    (:`0`
      (goto _label)))
  (set `self.Message` (`KismetStringLibrary.Concat_StrStr` "Добавлен итератор в стэк " "№" (`KismetStringLibrary.Conv_IntToString` (`KismetArrayLibrary.Array_Length` (`self.StackIter`)))))
  (`/Game/blueprints/Robot_sort/UI/RobotWidgetBase.UpDate` (`self.UI`))
  (`KismetArrayLibrary.Array_Add` (`self.StackIter`) _tempit)
  (`KismetArrayLibrary.Array_Add` _loopstack (make `IntVector` _tempit _output _globaliter))
  (`KismetSystemLibrary.PrintString` (`KismetStringLibrary.Concat_StrStr` "Loop  " (`KismetStringLibrary.Conv_IntToString` _tempit) (`KismetStringLibrary.Conv_IntToString` _output)))
  (set `self.Message` (`KismetStringLibrary.Concat_StrStr` "Iter#" (`KismetStringLibrary.Conv_IntToString` (`KismetArrayLibrary.Array_LastIndex` (`self.StackIter`))) " = " (`KismetStringLibrary.Conv_IntToString` _tempit)))
  (`/Game/blueprints/Robot_sort/UI/RobotWidgetBase.UpDate` (`self.UI`))
  (return _output_x))

(fn `fEndLoop`
  (returns (X :type Integer) (ReturnValue :type Boolean))
  (bind _loopstack (`self.LoopStack`))
  (bind _stackiter (`self.StackIter`))
  (bind _returnvalue (`KismetArrayLibrary.Array_LastIndex` _loopstack))
  (bind (_output_x _output_y _output_z) (break `IntVector` (`|GetArrayItem` _loopstack _returnvalue)))
  (if (`KismetArrayLibrary.Array_IsNotEmpty` _loopstack)
    (bind _result (`/Engine/EditorBlueprintResources/StandardMacros.IncrementInt` _output_x)
      (:`  `
        (set `self.Message` (`KismetStringLibrary.Concat_StrStr` "Iter#" (`KismetStringLibrary.Conv_IntToString` _returnvalue) " = " (`KismetStringLibrary.Conv_IntToString` _output_x)))
        (`/Game/blueprints/Robot_sort/UI/RobotWidgetBase.UpDate` (`self.UI`))
        (`KismetArrayLibrary.Array_Set` (`self.StackIter`) _returnvalue _result)
        (if (< _result _output_y)
          (set `self.GlobalIter` _output_z)
          (return _output_x true)
          (else
            (`KismetSystemLibrary.PrintString` (`KismetStringLibrary.Concat_StrStr` "Remove from steck " (`KismetStringLibrary.Conv_IntToString` _returnvalue)))
            (`KismetArrayLibrary.Array_Remove` _loopstack _returnvalue)
            (`KismetArrayLibrary.Array_Remove` _stackiter (`KismetArrayLibrary.Array_LastIndex` _stackiter)))))))
  (return 0 false))

(fn `fMin`
  (locals (T1 :type Integer :default 0) (T2 :type Integer :default 0))
  (bind _returnvalue (`KismetMathLibrary.SelectInt` (`local.T2`) (`local.T1`) (< (`KismetMathLibrary.GetMaxElement` (`.BoxExtent` (`KismetSystemLibrary.GetComponentBounds` (`|GetArrayItem` (`self.Array`) (`local.T2`))))) (`KismetMathLibrary.GetMaxElement` (`.BoxExtent` (`KismetSystemLibrary.GetComponentBounds` (`|GetArrayItem` (`self.Array`) (`local.T1`))))))))
  (bind _newparam (`self.IterOrConst`))
  (bind _output_get (set `local.T1` _newparam))
  (set `self.Message` (`KismetStringLibrary.Concat_StrStr` "Сравниваем Obj" (`KismetStringLibrary.Conv_IntToString` _output_get)))
  (`/Game/blueprints/Robot_sort/UI/RobotWidgetBase.UpDate` (`self.UI`))
  (bind _newparam_2 (`self.IterOrConst`))
  (bind _output_get_2 (set `local.T2` _newparam_2))
  (set `self.Message` (`KismetStringLibrary.Concat_StrStr` " c Obj" (`KismetStringLibrary.Conv_IntToString` _output_get_2)))
  (`/Game/blueprints/Robot_sort/UI/RobotWidgetBase.UpDate` (`self.UI`))
  (set `self.Message` (`KismetStringLibrary.Concat_StrStr` "Temp = " (`KismetStringLibrary.Conv_IntToString` _returnvalue)))
  (`/Game/blueprints/Robot_sort/UI/RobotWidgetBase.UpDate` (`self.UI`))
  (set `self.Temp ` _returnvalue))

(fn `fTEq`
  (bind _newparam (`self.IterOrConst`))
  (`KismetSystemLibrary.PrintString` (`KismetStringLibrary.Conv_IntToString` _newparam))
  (set `self.Temp ` _newparam))

(fn `IterOrConst`
  (returns (NewParam :type Integer))
  (locals (T :type Integer))
  (bind _output_get (set `self.GlobalIter` (+ (stale _output_get) 2)))
  (switch `int` (`|GetArrayItem` (`self.Commands`) (- (`self.GlobalIter`) 2))
    (:`Default`
      _)
    (:`-1`
      (return (`self.Temp `)))
    (:`0`
      _))
  (return (`|GetArrayItem` (`self.StackIter`) (`|GetArrayItem` (`self.Commands`) (- (`self.GlobalIter`) 1)))))

(fn `UserConstructionScript`)