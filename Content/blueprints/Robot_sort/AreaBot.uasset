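; AreaBot is a robot sorting puzzle area that opens a flipbook door when its check passes.
; Overlap by BP_Anton shows a RobotUI linked to the area and its child Robotsort; leaving hides it.
; Reload recreates the robot at its current transform and relinks the UI.
; The first Reload starts a two-second polling loop comparing X positions and bounds heights, which plays the door and removes Box1 on success.
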(event `self.Box.OnComponentBeginOverlap`
  (params (OverlappedComponent :type "PrimitiveComponent Object Reference") (OtherActor :type "Actor Object Reference") (OtherComp :type "PrimitiveComponent Object Reference") (OtherBodyIndex :type Integer) (bFromSweep :type Boolean) (SweepResult :type "HitResult Structure (by ref)"))
  (bind _asrobotsort (cast `/Game/blueprints/Robot_sort/Robotsort` (`ChildActorComponent.ChildActor` (`self.Robotsort`)) :!pure true))
  (bind _asbp_anton (cast `/Game/blueprints/Characters/Anton/BP_Anton` OtherActor))
  (`|ExecutionSequence`
    (:`then_0`
      (`/Engine/EditorBlueprintResources/StandardMacros.DoOnce` false
        (:`Completed`
          (bind _returnvalue (`|CreateWidget` "/Game/blueprints/Robot_sort/UI/RobotUI.RobotUI_C" (`Pawn.GetLocalViewingPlayerController` _asbp_anton)))
          (bind _output_get (set `self.UI` _returnvalue)))))
    (:`then_1`
      (bind _output_get_2 (set `/Game/blueprints/Robot_sort/Robotsort.UI` _output_get _asrobotsort))
      (set `/Game/blueprints/Robot_sort/UI/RobotUI.Area` self _output_get_2)
      (set `/Game/blueprints/Robot_sort/UI/RobotUI.Bot` _asrobotsort _output_get_2)
      (`UserWidget.AddToViewport` (`self.UI`) 0))))

(event `self.Box.OnComponentEndOverlap`
  (params (OverlappedComponent :type "PrimitiveComponent Object Reference") (OtherActor :type "Actor Object Reference") (OtherComp :type "PrimitiveComponent Object Reference") (OtherBodyIndex :type Integer))
  (`Widget.RemoveFromParent` (`self.UI`)))

(event `Reload`
  (bind _robotsort (`self.Robotsort`))
  (bind _asrobotsort (cast `/Game/blueprints/Robot_sort/Robotsort` (`ChildActorComponent.ChildActor` (`self.Robotsort`)) :!pure true))
  (set `self.Trans` (`self.GetTransform` (`ChildActorComponent.ChildActor` _robotsort)))
  (`ActorComponent.K2_DestroyComponent` _robotsort)
  (bind _returnvalue (`AddComponent|NODE_AddChildActorComponent-0`))
  (bind _output_get (set `self.Robotsort` _returnvalue))
  (`ChildActorComponent.SetChildActorClass` _returnvalue "/Game/blueprints/Robot_sort/Robotsort.Robotsort_C")
  (`ChildActorComponent.SetChildActorClass` _output_get "/Game/blueprints/Robot_sort/Robotsort.Robotsort_C")
  (`self.K2_SetActorTransform` (`ChildActorComponent.ChildActor` _output_get) (`self.Trans`) false false)
  (bind _output_get_2 (set `/Game/blueprints/Robot_sort/Robotsort.UI` (`self.UI`) _asrobotsort))
  (bind _output_get_3 (set `/Game/blueprints/Robot_sort/UI/RobotUI.Bot` _asrobotsort _output_get_2))
  (`/Engine/EditorBlueprintResources/StandardMacros.DoOnce` false
    (:`Completed`
      (bind _newparam (`self.Check` (`/Game/blueprints/Robot_sort/Robotsort.Array` _output_get_3) :!label _label))
      (if _newparam
        (`PaperFlipbookComponent.Play` (`self.dverFlipBook`))
        (`ActorComponent.K2_DestroyComponent` (`self.Box1`))
        (else
          (`KismetSystemLibrary.Delay` 2.0)
          (goto _label))))))

(fn `Check`
  (params (Array :type "Array of PaperSpriteComponent Object Reference"))
  (returns (NewParam :type Boolean))
  (locals (Flag :type Boolean))
  (bind _flag (`local.Flag`))
  (for _array_element Array
    (for _array_element_2 (`self.Array`)
      (bind _returnvalue_x (`KismetMathLibrary.BreakVector` (`SceneComponent.K2_GetComponentLocation` _array_element)))
      (bind _returnvalue_x_2 (`KismetMathLibrary.BreakVector` (`SceneComponent.K2_GetComponentLocation` _array_element_2)))
      (bind _output_get (set `local.Flag` (and (== _returnvalue_x _returnvalue_x_2) (== (.z (`.BoxExtent` (`KismetSystemLibrary.GetComponentBounds` _array_element_2))) (.z (`.BoxExtent` (`KismetSystemLibrary.GetComponentBounds` _array_element)))))))
      (if _output_get
        (break)))
    (if (not _flag)
      (break)))
  (return _flag))

(fn `UserConstructionScript`
  (set `self.Array` (`|MakeArray` (`self.Stone_1`) (`self.Stone_2`) (`self.Stone_3`) (`self.Stone_4`) (`self.Stone_5`)))
  (`PaperFlipbookComponent.Stop` (`self.dverFlipBook`))
  (`PaperFlipbookComponent.SetLooping` (`self.dverFlipBook`) false)
  (`PaperFlipbookComponent.SetLooping` (`self.dverFlipBook`) false))