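; BP_SHIP is a spline-shaped enemy hazard that damages the player's BP_Anton character on contact.
; On overlap it deals fixed damage, then repeats each second while the hero remains overlapping.
; The construction script tiles Paper2D sprite components along ShipSpline at midpoints of equal steps derived from the Ok variable.
; Logic to fit a box to the spline's span exists but is disconnected.
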(event `self.ReceiveBeginPlay`
  (bind _asbp_hero (cast `/Game/blueprints/Characters/Anton/BP_Anton` (`GameplayStatics.GetPlayerCharacter` 0)))
  (set `self.BP_hero` _asbp_hero))

(event `self.ReceiveActorBeginOverlap`
  (params (OtherActor :type "Actor Object Reference"))
  (bind _bp_hero (`self.BP_hero`))
  (if (== OtherActor _bp_hero)
    (`GameplayStatics.ApplyDamage` _bp_hero 20.0 :!label _label)
    (`KismetSystemLibrary.Delay` 1.0)
    (if (`self.IsOverlappingActor` _bp_hero)
      (goto _label))))

(fn `UserConstructionScript`
  (locals (NewLocalVar :type "Float (single-precision)" :default 0.0))
  (set `self.NewVar` (/ (`self.ok`) 10.0))
  (for _index (range (+ (`KismetMathLibrary.FTrunc` (/ (`SplineComponent.GetSplineLength` (`self.ship spline`)) (`self.NewVar`))) 1))
    (bind _returnvalue (`AddComponent|NODE_AddPaperSpriteComponent-0`))
    (`SceneComponent.K2_SetRelativeLocation` _returnvalue (/ (+ (`SplineComponent.GetLocationAtDistanceAlongSpline` (`self.ship spline`) (* (+ _index 1) (`self.NewVar`)) "Local") (`SplineComponent.GetLocationAtDistanceAlongSpline` (`self.ship spline`) (* _index (`self.NewVar`)) "Local")) (2.0 2.0 2.0)) false false)))