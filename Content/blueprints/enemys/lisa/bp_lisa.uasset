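; BP_Lisa is a side-view sprite enemy that walks constantly along X and hurts the player on touch.
; Tick drives movement from a direction flag, which Revers toggles while flipping the sprite; nothing here calls Revers.
; Overlapping the cached BP_Anton player applies damage, launches Lisa away from them and pauses walking for two seconds.
; An older counter-based patrol remains disconnected, and Follow is an empty stub.
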(event `self.ReceiveBeginPlay`
  (bind _asbp_anton (cast `/Game/blueprints/Characters/Anton/BP_Anton` (`GameplayStatics.GetPlayerCharacter` 0) :!label _label)
    (:`then`
      (set `self.BP_hero` _asbp_anton))
    (:`CastFailed`
      (`KismetSystemLibrary.Delay` 2.0)
      (goto _label))))

(event `self.ReceiveTick`
  (params (DeltaSeconds :type "Float (single-precision)"))
  (if (not (`self.Is Movement Lock`))
    (`self.AddMovementInput` (`KismetMathLibrary.MakeVector` (`KismetMathLibrary.SelectFloat` -1.0 1.0 (`self.Revers_0`))))))

(event `self.ReceiveActorBeginOverlap`
  (params (OtherActor :type "Actor Object Reference"))
  (bind _returnvalue_x (`KismetMathLibrary.BreakVector` (`SceneComponent.K2_GetComponentLocation` (`self.Sprite`))))
  (bind _returnvalue_x_2 (`KismetMathLibrary.BreakVector` (`SceneComponent.K2_GetComponentLocation` (`PaperCharacter.Sprite` (`self.BP_hero`)))))
  (if (== OtherActor (`self.BP_hero`))
    (`GameplayStatics.ApplyDamage` (`self.BP_hero`) (`self.Damage`) null self)
    (`self.LaunchCharacter` (`KismetMathLibrary.SelectVector` (-500.0 0.0 0.0) (500.0 0.0 0.0) (> _returnvalue_x_2 _returnvalue_x)) true)
    (set `self.Is Movement Lock` true)
    (`KismetSystemLibrary.Delay` 2.0)
    (set `self.Is Movement Lock` false)))

(event `Follow`)

(event `self.CapsuleComponent.OnComponentHit`
  (params (HitComponent :type "PrimitiveComponent Object Reference") (OtherActor :type "Actor Object Reference") (OtherComp :type "PrimitiveComponent Object Reference") (NormalImpulse :type "Vector Structure") (Hit :type "HitResult Structure (by ref)")))

(fn `Revers`
  (bind _output_get (set `self.Revers_0` (not (stale _output_get))))
  (`SceneComponent.K2_SetRelativeRotation` (`self.Sprite`) (`KismetMathLibrary.MakeRotator` 0.0 0.0 (`KismetMathLibrary.SelectFloat` 180.0 0.0 _output_get)) false false)
  (return))

(fn `UserConstructionScript`)