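; BP_Sosulka is an icicle (sosulka) Blueprint, filed with the enemies, that plays an animation and removes itself when opened.
; On BeginPlay it runs the parent logic, then casts its UI widget to FatherUI and registers itself as that widget's Parent.
; The Open event switches the flipbook component to another animation, waits for that flipbook's length and destroys the actor.
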(event `self.ReceiveBeginPlay`
  (`parent.ReceiveBeginPlay`)
  (set `/Game/blueprints/enemys/FatherUI.Parent` self (cast `/Game/blueprints/enemys/FatherUI` (`self.UIWidget`) :!pure true)))

(event `Open`
  (bind _sosulka2 (`self.sosulka2`))
  (`PaperFlipbookComponent.SetFlipbook` _sosulka2 "/Game/assets/sosulka1.sosulka1")
  (`KismetSystemLibrary.Delay` (`PaperFlipbookComponent.GetFlipbookLength` _sosulka2))
  (`self.K2_DestroyActor`))

(fn `UserConstructionScript`
  (`parent.UserConstructionScript`))