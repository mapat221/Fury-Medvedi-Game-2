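; End1 is an end trigger actor that fades in or out an image in the End2 UI when the hero overlaps it.
; The overlap passes a DoOnce and plays a Timeline, whose track drives the render opacity of the widget's Image0.
; Each Timeline update also disables the hero's player input.
; A disconnected branch that would move a PaperSprite vertically from the same track never runs.
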(event `self.ReceiveActorBeginOverlap`
  (params (OtherActor :type "Actor Object Reference"))
  (`parent.ReceiveActorBeginOverlap` OtherActor)
  (if (== OtherActor (`self.BP_hero`))
    (`/Engine/EditorBlueprintResources/StandardMacros.DoOnce` false
      (:`Completed`
        (bind (_direction _newtrack_0) (`Timeline|Timeline` :!via `PlayFromStart`)
          (:`Update`
            (`Widget.SetRenderOpacity` (`/Game/blueprints/enemys/End2.Image_0` (cast `/Game/blueprints/enemys/End2` (`self.UIWidget`) :!pure true)) _newtrack_0)
            (`self.DisableInput` (`self.BP_hero`) (`GameplayStatics.GetPlayerController` 0))))))))

(event `self.ReceiveActorEndOverlap`
  (params (OtherActor :type "Actor Object Reference")))

(fn `UserConstructionScript`
  (`parent.UserConstructionScript`))