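; Base game mode that sets up the player's session: ability save, audio, graphics quality, HUD and pause menu.
; On BeginPlay it loads or creates the Save_Base ability save, caches BP_Anton and re-applies an unlocked double jump.
; AllowDJump saves that unlock and raises the jump count.
; Quality settings run as console command arrays through SetSet, and Escape flip-flops the menu widget on and off screen.
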(event `LoadDataFromSave`
  (if (`/Game/blueprints/Characters/Save_Base.HaveDJump` (`self.As Save Base`))
    (`self.AllowDJump`)))

(event `self.ReceiveBeginPlay`
  (bind _returnvalue (`GameplayStatics.LoadGameFromSlot` (`self.SaveAbilki`)))
  (bind _assave_base (cast `/Game/blueprints/Characters/Save_Base` _returnvalue)
    (:`then`
      (set `self.As Save Base` _assave_base))
    (:`CastFailed`
      (bind _returnvalue_2 (`GameplayStatics.CreateSaveGameObject` "/Game/blueprints/Characters/Save_Base.Save_Base_C"))
      (set `self.As Save Base` _returnvalue_2)))
  (set `self.As BP Anton` (cast `/Game/blueprints/Characters/Anton/BP_Anton` (`GameplayStatics.GetPlayerPawn` 0) :!pure true))
  (`self.LoadDataFromSave`)
  (bind _returnvalue_3 (`AddComponent|NODE_AddAudioComponent-0`))
  (`AudioComponent.SetSound` _returnvalue_3 (`self.Sound`))
  (`|ExecutionSequence`
    (:`then_0`
      (`self.SetSet` (`self.PostQ`)))
    (:`then_1`
      (`self.SetSet` (`self.ShadowQ`)))
    (:`then_2`
      (`self.SetSet` (`self.EffectsQ`)))
    (:`then_3`
      (set `PlayerController.bShowMouseCursor` true (`GameplayStatics.GetPlayerController` 0))
      (`|ExecutionSequence`
        (:`then_0`
          (bind _returnvalue_4 (`|CreateWidget` "/Game/blueprints/Characters/hood/healthbar.healthbar_C"))
          (`UserWidget.AddToViewport` _returnvalue_4 0)
          (bind _returnvalue_5 (`|CreateWidget` "/Game/blueprints/EscMenuWidget.EscMenuWidget_C"))
          (set `self.EscMenu` _returnvalue_5))))))

(event `AllowDJump`
  (bind _as_save_base (`self.As Save Base`))
  (set `/Game/blueprints/Characters/Save_Base.HaveDJump` true _as_save_base)
  (`GameplayStatics.SaveGameToSlot` _as_save_base (`self.SaveAbilki`))
  (set `Character.JumpMaxCount` 2 (`self.As BP Anton`)))

(event `Key|Escape`
  (params (Key :type "Key Structure"))
  (bind _escmenu (`self.EscMenu`))
  (:`Pressed`
    (`/Engine/EditorBlueprintResources/StandardMacros.FlipFlop`
      (:`A`
        (`UserWidget.AddToViewport` _escmenu 0))
      (:`B`
        (`Widget.RemoveFromParent` _escmenu)))))

(fn `SetSet`
  (params (Array :type "Array of String"))
  (for _array_element Array
    (`KismetSystemLibrary.ExecuteConsoleCommand` _array_element null)))

(fn `UserConstructionScript`)